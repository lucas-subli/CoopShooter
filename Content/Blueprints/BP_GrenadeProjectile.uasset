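; Grenade projectile actor that explodes on a short fixed fuse after spawning.
; BeginPlay waits one second, then calls Explode, which spawns a cartoon explosion particle and applies full radial damage within DamageRadius, credited to the instigator's controller.
; It also draws a debug sphere showing the blast radius before destroying itself.
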(event Custom|Explode
  (bind _returnvalue (Transformation|GetActorLocation))
  (Effects|SpawnEmitteratLocation "/Game/ImpactFX/ParticleSystems/JangaFX/Par_Cartoon_Explosion_01.Par_Cartoon_Explosion_01" _returnvalue)
  (Game|Damage|ApplyRadialDamage 5e+01 _returnvalue (Variables|Default|GetDamageRadius) 0 0 self (Game|GetInstigatorController) true "ECC_Visibility")
  (Rendering|Debug|DrawDebugSphere (Transformation|GetActorLocation) (Variables|Default|GetDamageRadius) 12 "(R=0.609375,G=0.029860,B=0.015869,A=1.000000)" 2.0 2.0)
  (Actor|DestroyActor))

(event EventBeginPlay
  (Utilities|FlowControl|Delay 1.0)
  (CallFunction|Explode))

(fn ConstructionScript)